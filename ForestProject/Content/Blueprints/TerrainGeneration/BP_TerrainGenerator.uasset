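; Terrain generator Blueprint that builds a grid-based procedural mesh landscape with collision on BeginPlay.
; GenerateTerrain samples an XSize by YSize vertex grid spaced by CellSize, setting height from two summed, scaled 1D Perlin noise samples, one per axis.
; It adds two triangles per cell, creates the TerrainMesh section without supplying normals or UVs, and applies the MI_ProcGrid material.
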(event EventBeginPlay
  (CallFunction|GenerateTerrain))

(fn ConstructionScript)

(fn GenerateTerrain
  (bind _xsize (Variables|Default|GetXSize))
  (bind _triangles (Variables|Default|GetTriangles))
  (bind _cell_size (Variables|Default|GetCell%20Size))
  ;[0 0.1288 1 1 31] Sampling points
  (for _index (range 0 (- (Variables|Default|GetYSize) 1))
    (for _index_2 (range 0 (- (Variables|Default|GetXSize) 1))
      (Utilities|Array|Add (Variables|Default|GetVertices) (Math|Vector|MakeVector (* _cell_size _index_2) (* _cell_size _index) (* (+ (Class|KismetMathLibrary|PerlinNoise1D (+ (* _cell_size _index_2) 0.1)) (Class|KismetMathLibrary|PerlinNoise1D (+ (* _cell_size _index) 0.1))) 5e+02)))))
  ;[0 1 0.03548 1 31] Sampling Tris
  (for _index_3 (range 0 (- (Variables|Default|GetYSize) 2))
    (for _index_4 (range 0 (- (Variables|Default|GetXSize) 2))
      ;;[0 1 0.03232] Adding verticies from the bottom tri of the square
      (Utilities|Array|Add _triangles (+ _index_4 (* _index_3 _xsize)))
      (Utilities|Array|Add _triangles (+ (+ _index_4 (* _index_3 _xsize)) _xsize))
      (Utilities|Array|Add _triangles (+ (+ _index_4 (* _index_3 _xsize)) 1))
      ;;[0 0.4072 0.01298] Adding verticies from the top tri of the square
      (Utilities|Array|Add _triangles (+ (+ _index_4 (* _index_3 _xsize)) _xsize))
      (Utilities|Array|Add _triangles (+ (+ (+ _index_4 (* _index_3 _xsize)) _xsize) 1))
      (Utilities|Array|Add _triangles (+ (+ _index_4 (* _index_3 _xsize)) 1))))
  ;[1 1 1 1 31] Generating Mesh
  (Class|ProceduralMeshComponent|CreateMeshSectionLinearColor (Variables|Default|GetTerrainMesh) 0 (Variables|Default|GetVertices) (Variables|Default|GetTriangles) 0 0 0 0 0 0 0 true false)
  (Rendering|Material|SetMaterial (Variables|Default|GetTerrainMesh) 0 "/Engine/OpenWorldTemplate/LandscapeMaterial/MI_ProcGrid.MI_ProcGrid"))