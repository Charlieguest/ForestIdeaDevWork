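; Procedural terrain generator actor that calls GenerateTerrain for each cell of an X by Y section grid on BeginPlay.
; GenerateTerrain is not defined here; the Blueprint version, GenerateTerrainBP, is left unconnected.
; That version sums three noise octaves, each a product of two 1D Perlin samples, for height.
; It builds padded tiles, computes tangents, then trims the border so normals match across procedural mesh sections.
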(event EventBeginPlay
  (for _index (range 0 (- (Variables|Default|GetNumOfSectionsY) 1))
    (for _index_2 (range 0 (- (Variables|Default|GetNumOfSectionsX) 1))
      (Class|WorldGenerator|GenerateTerrain _index_2 _index))))

(fn ConstructionScript)

(fn GenerateTerrainBP
  (params (XSectionIndex :type Integer) (YSectionIndex :type Integer))
  (bind _xvertexcount (Variables|Default|GetXVertexCount))
  (bind _triangles (LocalVariables|GetTriangles))
  (bind _cellsize (Variables|Default|GetCellSize))
  (bind _meshsectionindex (Variables|Default|GetMeshSectionIndex))
  (bind _tileoffset (LocalVariables|GetTileOffset))
  (bind _returnvalue (+ _xvertexcount 2))
  ;[0 0.1288 1 1 31] Sampling points and UVs
  (|CalculatingSectionOffsetBP)
  ;;[0.872 0 1] Getting Vertices around the tiles so that the end parts can connect
  (for _index (range -1 (Variables|Default|GetYVertexCount))
    (for _index_2 (range -1 (Variables|Default|GetXVertexCount))
      (Utilities|Array|Add (LocalVariables|GetVerticies) (Math|Vector|MakeVector (+ (.x _tileoffset) (* _cellsize _index_2)) (+ (.y _tileoffset) (* _cellsize _index)) (CallFunction|GetHeightBP (+ (.x _tileoffset) (* _cellsize _index_2)) (+ (.y _tileoffset) (* _cellsize _index)))))
      (Utilities|Array|Add (LocalVariables|GetUVs) (Math|Vector2D|MakeVector2D (.ReturnValue (|CalculateUVsBP _index_2 _index)) (.ReturnValue2 (|CalculateUVsBP _index_2 _index))))))
  ;[0 1 0.03548 1 31] Sampling Tris
  (for _index_3 (range 0 (Variables|Default|GetYVertexCount))
    (for _index_4 (range 0 (Variables|Default|GetXVertexCount))
      ;;[0 1 0.03232] Adding verticies from the bottom tri of the square
      (Utilities|Array|Add _triangles (+ _index_4 (* _index_3 _returnvalue)))
      (Utilities|Array|Add _triangles (+ (+ _index_4 (* _index_3 _returnvalue)) _returnvalue))
      (Utilities|Array|Add _triangles (+ (+ _index_4 (* _index_3 _returnvalue)) 1))
      ;;[0 0.4072 0.01298] Adding verticies from the top tri of the square
      (Utilities|Array|Add _triangles (+ (+ _index_4 (* _index_3 _returnvalue)) _returnvalue))
      (Utilities|Array|Add _triangles (+ (+ (+ _index_4 (* _index_3 _returnvalue)) _returnvalue) 1))
      (Utilities|Array|Add _triangles (+ (+ _index_4 (* _index_3 _returnvalue)) 1))))
  ;[1 1 1 1 31] Generating Mesh
  (bind (_verticies _triangles_2 _normals _uvs _tangents) (CallFunction|GetSubsetBP (LocalVariables|GetVerticies) (LocalVariables|GetTriangles) (LocalVariables|GetUVs)))
  (Class|ProceduralMeshComponent|CreateMeshSectionLinearColor (Variables|Default|Get_BPProcTerrain) _meshsectionindex _verticies _triangles_2 _normals _uvs 0 0 0 0 _tangents true false)
  (Rendering|Material|SetMaterial (Variables|Default|Get_BPProcTerrain) _meshsectionindex "/Game/Materials/Terrain/MI_TerrainMaterial.MI_TerrainMaterial")
  (Math|Integer|IncrementInt (Variables|Default|GetMeshSectionIndex)))

(fn GetHeightBP
  (params (In%20X :type Float%20%28double-precision%29) (In%20Y :type Float%20%28double-precision%29))
  (return (+ (CallFunction|PerlinNoise2DBP In%20X In%20Y 0.0001 0.0001 1e+04) (CallFunction|PerlinNoise2DBP In%20X In%20Y 0.001 0.001 6e+02) (CallFunction|PerlinNoise2DBP In%20X In%20Y 0.01 0.01 1.5e+02))))

(fn PerlinNoise2DBP
  (params (In%20X :type Float%20%28double-precision%29) (In%20Y :type Float%20%28double-precision%29) (In%20Scale%20X :type Float%20%28double-precision%29) (In%20Scale%20Y :type Float%20%28double-precision%29) (Amplitude :type Float%20%28double-precision%29))
  (return (* (* (Class|KismetMathLibrary|PerlinNoise1D (+ (* In%20X In%20Scale%20X) 0.1)) (Class|KismetMathLibrary|PerlinNoise1D (+ (* In%20Y In%20Scale%20Y) 0.1))) Amplitude)))

(fn GetSubsetBP
  (params (InVertices :type Array%20of%20Vectors) (InTriangles :type Array%20of%20Integers) (InUVs :type Array%20of%20Vector%202D%20Structures))
  (bind _xvertexcount (Variables|Default|GetXVertexCount))
  (bind _outtriangles (LocalVariables|GetOutTriangles))
  (bind (_normals _tangents) (Class|KismetProceduralMeshLibrary|CalculateTangentsforMesh InVertices InTriangles InUVs))
  (LocalVariables|SetBig%20Normals _normals)
  (LocalVariables|SetBig%20Tangents _tangents)
  (for _index (range -1 (Variables|Default|GetYVertexCount))
    (for _index_2 (range -1 (Variables|Default|GetXVertexCount))
      ;[1 1 1] Filtering out outer edge of the tile
      (if (Math|Boolean|ANDBoolean (> _index_2 -1) (< _index_2 (Variables|Default|GetXVertexCount)) (> _index -1) (< _index (Variables|Default|GetYVertexCount)))
        ;[0 0.1928 1] Getting the original values for the original tile to generate
        (Utilities|Array|Add (LocalVariables|GetOutVerticies) (Utilities|Array|Get(acopy) InVertices (LocalVariables|GetIndex)))
        (Utilities|Array|Add (LocalVariables|GetOutUVs) (Utilities|Array|Get(acopy) InUVs (LocalVariables|GetIndex)))
        (Utilities|Array|Add (LocalVariables|GetOutNormals) (Utilities|Array|Get(acopy) (LocalVariables|GetBig%20Normals) (LocalVariables|GetIndex)))
        (Utilities|Array|Add (LocalVariables|GetOutTangents) (Utilities|Array|Get(acopy) (LocalVariables|GetBig%20Tangents) (LocalVariables|GetIndex))))
      (Math|Integer|IncrementInt (LocalVariables|GetIndex))))
  ;[0 1 0.03548 1 31] Sampling Tris for original tile
  (for _index_3 (range 0 (- (Variables|Default|GetYVertexCount) 2))
    (for _index_4 (range 0 (- (Variables|Default|GetXVertexCount) 2))
      ;;[0 1 0.03232] Adding verticies from the bottom tri of the square
      (Utilities|Array|Add _outtriangles (+ _index_4 (* _index_3 _xvertexcount)))
      (Utilities|Array|Add _outtriangles (+ (+ _index_4 (* _index_3 _xvertexcount)) _xvertexcount))
      (Utilities|Array|Add _outtriangles (+ (+ _index_4 (* _index_3 _xvertexcount)) 1))
      ;;[0 0.4072 0.01298] Adding verticies from the top tri of the square
      (Utilities|Array|Add _outtriangles (+ (+ _index_4 (* _index_3 _xvertexcount)) _xvertexcount))
      (Utilities|Array|Add _outtriangles (+ (+ (+ _index_4 (* _index_3 _xvertexcount)) _xvertexcount) 1))
      (Utilities|Array|Add _outtriangles (+ (+ _index_4 (* _index_3 _xvertexcount)) 1))))
  (return (LocalVariables|GetOutVerticies) (LocalVariables|GetOutTriangles) (LocalVariables|GetOutNormals) (LocalVariables|GetOutUVs) (LocalVariables|GetOutTangents)))